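; Pickup actor that acts as a Collectible, Key or Map based on ItemType, destroying itself when the ThirdPersonCharacter overlaps it.
; Overlap runs a per-type macro: each prints a message, and Key also sets GotKey on the referenced Door.
; The construction script selects the Visual mesh by type, though every branch currently assigns None.
; Tick spins the Visual by a fixed per-frame amount without delta-time scaling; an offset timeline is left unconnected.
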(event EventBeginPlay)

(event Collision|EventActorBeginOverlap
  (params (OtherActor :type Actor%20Object%20Reference))
  (bind _asthird_person_character (Utilities|Casting|CastToThirdPersonCharacter OtherActor)
    (:then
      (Variables|Default|SetPlayer _asthird_person_character)
      (switch Utilities|FlowControl|Switch|SwitchonPickupTypes (Variables|Default|GetItemType)
        (:NewEnumerator0
          (Utilities|CollectibleMacro
            (:NewParam2
              _)))
        (:NewEnumerator1
          (Utilities|KeyMacro
            (:NewParam2
              _)))
        (:NewEnumerator2
          (Utilities|MapMacro
            (:NewParam
              _))))
      (Development|PrintString "Goodbye!")
      (Actor|DestroyActor))
    (:CastFailed
      (Development|PrintString "Not the Player"))))

(event EventTick
  (params (DeltaSeconds :type Float%20%28single-precision%29))
  (Transformation|AddWorldRotation (Variables|Default|GetVisual) (Math|Rotator|MakeRotator 0.0 0.0 (Variables|Default|GetRotationSpeedPerSecond)) false false))

(fn ConstructionScript
  (Utilities|FlowControl|Sequence
    (:then_0
      (switch Utilities|FlowControl|Switch|SwitchonPickupTypes (Variables|Default|GetItemType)
        (:NewEnumerator0
          (Variables|Default|SetMeshes 0))
        (:NewEnumerator1
          (Variables|Default|SetMeshes 0))
        (:NewEnumerator2
          (Variables|Default|SetMeshes 0))))
    (:then_1
      (Components|StaticMesh|SetStaticMesh (Variables|Default|GetVisual) (Variables|Default|GetMeshes)))))