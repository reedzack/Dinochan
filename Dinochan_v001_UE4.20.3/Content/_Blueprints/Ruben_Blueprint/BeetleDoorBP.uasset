(event EventBeginPlay)

(event Collision|EventActorBeginOverlap
  (params (OtherActor :type Actor%20Object%20Reference))
  (Utilities|FlowControl|Gate true) ; enters at Open
)

(event EventTick
  (params (DeltaSeconds :type Float%20%28single-precision%29)))

(event Collision|EventActorEndOverlap
  (params (OtherActor :type Actor%20Object%20Reference))
  (Utilities|FlowControl|Gate true) ; enters at Close
)

(event Input|KeyboardEvents|E
  (params (Key :type Key%20Structure))
  (:Pressed
    (Utilities|FlowControl|Gate true
      (:Exit
        (if (Variables|Default|GetGotKey)
          (bind _newtrack_1 (Timeline|Timeline_0 Play)
            (:Update
              (Transformation|SetWorldRotation (Variables|Default|GetScene) (Math|Rotator|MakeRotator 0.0 _newtrack_1 0.0) false false)
              (Transformation|SetWorldRotation (Variables|Default|GetScene1) (Math|Rotator|MakeRotator 0.0 (* _newtrack_1 -1.0) 0.0) false false)))
          (else
            (Development|PrintString "You need a key")))))))

(fn ConstructionScript)