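; Pickup actor that acts as a Collectible, Key or Map based on ItemType, with the construction script assigning the matching placeholder mesh.
; Tick spins the mesh by a fixed yaw each frame and bobs it with a ping-pong Lerp; a leftover Timeline is unused.
; Overlap with the ThirdPersonCharacter runs a per-type macro, then destroys the pickup.
; Key flags its Door as GotKey and toggles that door's key visibility; Collectible and Map only print messages.
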(event EventBeginPlay)

(event Collision|EventActorBeginOverlap
  (params (OtherActor :type Actor%20Object%20Reference))
  (|OverlapWithPlayer OtherActor))

(event EventTick
  (params (DeltaSeconds :type Float%20%28single-precision%29))
  (Utilities|FlowControl|Sequence
    (:then_0
      (|RotateAnim))
    (:then_1
      (|BounceAnim DeltaSeconds))))

(fn ConstructionScript
  (Utilities|FlowControl|Sequence
    (:then_0
      (switch Utilities|FlowControl|Switch|SwitchonPickupTypes (Variables|Default|GetItemType)
        (:NewEnumerator0
          (Variables|Default|SetMeshes "/Game/1_Models/PlaceholderModels/PlaceHolder_Item.PlaceHolder_Item"))
        (:NewEnumerator1
          (Variables|Default|SetMeshes "/Game/1_Models/PlaceholderModels/PlaceHolder_Key.PlaceHolder_Key"))
        (:NewEnumerator2
          (Variables|Default|SetMeshes "/Game/1_Models/PlaceholderModels/PlaceHolder_Map.PlaceHolder_Map"))))
    (:then_1
      (Components|StaticMesh|SetStaticMesh (Variables|Default|GetVisual) (Variables|Default|GetMeshes)))))